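; BP_DoorWithKeys is a sliding door that opens when its key count matches the required total or, if pin-protected, when the pin is correct.
; Player overlap shows a HUD message and attempts opening, and leaving closes it, unless overlap is ignored.
; Enemy overlap also attempts opening.
; Switch on/off overrides add or remove keys, while a reversible timeline moves the door and two lights indicate lock state.
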(event `self.InteractCollision.OnComponentBeginOverlap`
  (params (OverlappedComponent :type "PrimitiveComponent Object Reference") (OtherActor :type "Actor Object Reference") (OtherComp :type "PrimitiveComponent Object Reference") (OtherBodyIndex :type Integer) (bFromSweep :type Boolean) (SweepResult :type "HitResult Structure (by ref)"))
  ;[1 1 1] show message and open door if player is close
  (`|ExecutionSequence`
    (:`then_0`
      (bind _asbp_ctr_player (cast `/Game/MyContent/Characters/BP_CTR_Player` OtherActor))
      (if (not (`self.IgnoreOverlap`))
        (`/Game/MyContent/Characters/UI/UI_PlayerHUD.SetDoorMessage` (`/Game/MyContent/Characters/BP_CTR_Player.PlayerHUD` _asbp_ctr_player) true (`self.DoorMessage`))
        (`self.OpenDoor`)))
    (:`then_1`
      (cast `/Game/MyContent/Characters/Enemies/BP_CTR_Enemy` OtherActor)
      (`self.OpenDoor`))))

(event `self.InteractCollision.OnComponentEndOverlap`
  (params (OverlappedComponent :type "PrimitiveComponent Object Reference") (OtherActor :type "Actor Object Reference") (OtherComp :type "PrimitiveComponent Object Reference") (OtherBodyIndex :type Integer))
  ;[1 1 1] remove message and close door when leaving
  (bind _asbp_ctr_player (cast `/Game/MyContent/Characters/BP_CTR_Player` OtherActor))
  (if (not (`self.IgnoreOverlap`))
    (`/Game/MyContent/Characters/UI/UI_PlayerHUD.SetDoorMessage` (`/Game/MyContent/Characters/BP_CTR_Player.PlayerHUD` _asbp_ctr_player) false (`self.DoorMessage`))
    (`self.CloseDoor`)))

(event `OpenDoor`
  ;[1 1 1] if pin protected dont worry about keys. if pin correct, open door
  (if (`self.IsPinProtected`)
    (if (`self.IsPinCorrect`)
      ;[1 1 1] open/close door flow
      (`self.SetLightColours` (`self.OpenLight`) :!label _label)
      (if (not (`self.isDoorOpen`))
        (set `self.isDoorOpen` true)
        (bind (_direction _alpha) (`Timeline|TL_OpenCloseDoor` :!label _label_2)
          (:`Update`
            (`SceneComponent.K2_SetRelativeLocation` (`self.Transform`) (`KismetMathLibrary.VLerp` (0.0 0.0 0.0) (`self.OpenLocation`) _alpha) false false)))))
    (else
      (bind _allkeyscollected (`self.AreAllKeysCollected`))
      (if _allkeyscollected
        (goto _label)
        (else
          (`self.SetLightColours` (`self.CloseLight`)))))))

(event `CloseDoor`
  ;[1 1 1] open/close door flow
  (if (`self.isDoorOpen`)
    (set `self.isDoorOpen` false)
    (goto _label_2 :!via `Reverse`)))

(fn `AddKey`
  (params (openOnUnlock :type Boolean))
  (`/Engine/EditorBlueprintResources/StandardMacros.IncrementInt` (`self.KeysCollected`)
    (:`  `
      (if openOnUnlock
        (`self.OpenDoor`)))))

(fn `AreAllKeysCollected`
  (returns (allKeysCollected :type Boolean))
  (return (== (`self.KeysToCollect`) (`self.KeysCollected`))))

(fn `Interact`
  (`parent.Interact`))

(fn `RemoveKey`
  (params (closeOnLock :type Boolean))
  (`/Engine/EditorBlueprintResources/StandardMacros.DecrementInt` (`self.KeysCollected`)
    (:`  `
      (if closeOnLock
        (`self.CloseDoor`)))))

(fn `SetLightColours`
  (params (NewLightColor :type "LinearColor Structure"))
  (`LightComponent.SetLightColor` (`self.DoorLightFront`) NewLightColor true)
  (`LightComponent.SetLightColor` (`self.DoorLightBack`) NewLightColor true))

(fn `SwitchedOff`
  (`parent.SwitchedOff`)
  (`self.SetLightColours` (`self.CloseLight`))
  (`self.RemoveKey` true))

(fn `SwitchedOn`
  (`parent.SwitchedOn`)
  (`self.AddKey` true))

(fn `UserConstructionScript`
  (bind _allkeyscollected (`self.AreAllKeysCollected`))
  (if _allkeyscollected
    (`self.SetLightColours` (`self.OpenLight`))
    (else
      (`self.SetLightColours` (`self.CloseLight`)))))