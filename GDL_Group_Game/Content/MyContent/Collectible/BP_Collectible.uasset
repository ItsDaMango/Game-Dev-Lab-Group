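; BP_Collectible is a pickup actor that removes itself from the world when an actor overlaps its InteractCollision component.
; The overlap event calls Collect, which currently just destroys the actor through OnDestroy without filtering the overlapping actor.
; Adding to the player's inventory widget is unfinished, disconnected logic noted as needing debugging.
; GetCollectibleDataForInventory exposes the item's class, max quantity and icon for inventory use.
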(event `self.InteractCollision.OnComponentBeginOverlap`
  (params (OverlappedComponent :type "PrimitiveComponent Object Reference") (OtherActor :type "Actor Object Reference") (OtherComp :type "PrimitiveComponent Object Reference") (OtherBodyIndex :type Integer) (bFromSweep :type Boolean) (SweepResult :type "HitResult Structure (by ref)"))
  (`self.collect` OtherActor))

(fn `collect`
  (params (otherActor :type "Actor Object Reference"))
  ;[1 1 1] for now destory... inventory needs debugging
  (`self.onDestroy`))

(fn `getCollectibleDataForInventory`
  (returns (ItemClass :type "Actor Class Reference") (MaxQuantity :type Integer) (ItemIcon :type "Texture2D Object Reference"))
  (return (`self.ItemClass`) (`self.MaxQuantity`) (`self.ItemIcon`)))

(fn `onDestroy`
  (`self.K2_DestroyActor`))

(fn `UserConstructionScript`)