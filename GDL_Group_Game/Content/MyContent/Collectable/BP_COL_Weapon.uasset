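; BP_COL_Weapon is a collectable weapon pickup that lets the player equip a weapon.
; On BeginPlay, WeaponToPickup sets the Weapon skeletal mesh from the WeaponPickup variable.
; When a BP_CTR_Player overlaps InteractCollision, it sets that player's EquipWeapon flag to true and destroys itself, without passing along which weapon was picked up.
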(event `self.ReceiveBeginPlay`
  (`self.WeaponToPickup`))

(event `self.InteractCollision.OnComponentBeginOverlap`
  (params (OverlappedComponent :type "PrimitiveComponent Object Reference") (OtherActor :type "Actor Object Reference") (OtherComp :type "PrimitiveComponent Object Reference") (OtherBodyIndex :type Integer) (bFromSweep :type Boolean) (SweepResult :type "HitResult Structure (by ref)"))
  (bind _asbp_ctr_player (cast `/Game/MyContent/Characters/BP_CTR_Player` OtherActor))
  (set `/Game/MyContent/Characters/BP_CTR_Player.EquipWeapon` true _asbp_ctr_player)
  (`self.K2_DestroyActor`))

(fn `UserConstructionScript`
  (`parent.UserConstructionScript`))

(fn `WeaponToPickup`
  (`SkeletalMeshComponent.SetSkeletalMeshAsset` (`self.Weapon`) (`self.WeaponPickup`)))