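; Interactible lever switch that reopens a linked door, DoorB, when switched on.
; SwitchedOn extends the parent switch logic: with a valid DoorB, it sets the door's reopen flags and calls Reverse on it.
; It then immediately fires SwitchOff, which restores those flags through SwitchedOff, and plays a timeline that rotates the lever mesh.
; Debug prints trace each step.
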(event `Switch Off`
  (`self.SwitchedOff`)
  (`KismetSystemLibrary.PrintString` "OFFF \n"))

(event `Lever`
  (bind (_direction _alpha) (`Timeline|TL_Lever` :!via `PlayFromStart`)
    (:`Update`
      (`SceneComponent.K2_SetRelativeRotation` (`self.StaticMesh1`) (`KismetMathLibrary.RLerp` (struct) (struct :`Roll` 80.0) _alpha) false false))))

(fn `SwitchedOff`
  (bind _doorb (`self.DoorB`))
  (`parent.SwitchedOff`)
  (set `/Game/MyContent/Interactibles/BP_INT_SS_DoorB.PlayerHasActivated` true _doorb)
  (set `/Game/MyContent/Interactibles/BP_INT_SS_DoorB.CanReopen` false _doorb))

(fn `SwitchedOn`
  (`parent.SwitchedOn`)
  (`self.DoorB`
    (:`then`
      (`KismetSystemLibrary.PrintString` "Hello")
      (set `/Game/MyContent/Interactibles/BP_INT_SS_DoorB.CanReopen` true (`self.DoorB`))
      (set `/Game/MyContent/Interactibles/BP_INT_SS_DoorB.PlayerHasActivated` false (`self.DoorB`))
      (`/Game/MyContent/Interactibles/BP_INT_SS_DoorB.Reverse` (`self.DoorB`))
      (`KismetSystemLibrary.PrintString` "Reopen Last Door")
      (`self.Switch Off`)
      (`self.Lever`))
    (:`else`)))

(fn `UserConstructionScript`
  (`parent.UserConstructionScript`))