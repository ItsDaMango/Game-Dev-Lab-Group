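; Interactable door Blueprint that slides its Door component between a stored Location and its relative origin on the TL_Door2 timeline.
; Open plays the timeline toward the origin after CloseDelay once the player has activated it, and Reverse runs it back after ReopenDelay when reopening is allowed.
; StopDoor halts the timeline only on the door flagged IsLastDoor.
; The construction script only calls the parent's.
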(event `StopDoor`
  (if (`self.IsLastDoor`)
    (bind (_direction _alpha) (`Timeline|TL_Door2` :!via `Stop` :!label _label)
      (:`Update`
        (`SceneComponent.K2_SetRelativeLocation` (`self.Door`) (`KismetMathLibrary.VLerp` (`self.Location`) (0.0 0.0 0.0) _alpha) false false)))))

(event `Open`
  (if (`self.PlayerHasActivated`)
    (`KismetSystemLibrary.Delay` (`self.CloseDelay`))
    (goto _label)))

(event `Reverse`
  (if (`self.CanReopen`)
    (`KismetSystemLibrary.Delay` (`self.ReopenDelay`))
    (goto _label :!via `Reverse`)))

(fn `UserConstructionScript`
  (`parent.UserConstructionScript`))