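; End-game lever switch that finishes the game once enough of the tracked enemies are gone.
; After a long delay at BeginPlay it starts a looping timer, apparently for CheckEnemiesAlive, which rebuilds a counter by adding invalid and subtracting valid enemy references.
; Switching on tests that counter against a threshold, then clears the check by function name, calls Lever and EndGame, and shows the player's GameOver HUD.
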(event `self.ReceiveBeginPlay`
  (`parent.ReceiveBeginPlay`)
  (`KismetSystemLibrary.Delay` 200.0)
  (`KismetSystemLibrary.K2_SetTimerDelegate` (`|CreateDelegate` :!event `CheckEnemiesAlive`) 2.0 true))

(fn `CheckEnemiesAlive`
  ;[1 1 1] Reset Counter
  (set `self.EnemiesCounter` 0)
  ;[1 1 1] Get All the enemies and check are they valid?
  (for _array_element (`self.Enemies`)
    (`/Engine/EditorBlueprintResources/StandardMacros.IsValid` _array_element
      (:`Is Valid`
        (`/Engine/EditorBlueprintResources/StandardMacros.DecrementInt` (`self.EnemiesCounter`)))
      (:`Is Not Valid`
        (`/Engine/EditorBlueprintResources/StandardMacros.IncrementInt` (`self.EnemiesCounter`)))))
  ;[1 1 1] If all are NOT valid, stop checking
  (if (>= (`self.EnemiesCounter`) 5)
    (`KismetSystemLibrary.K2_ClearTimer` null "CheckEnemiesAlive")))

(fn `SwitchedOff`
  (`parent.SwitchedOff`))

(fn `SwitchedOn`
  (`parent.SwitchedOn`)
  (if (>= (`self.EnemiesCounter`) 4)
    (`KismetSystemLibrary.K2_ClearTimer` null "CheckEnemiesAlive")
    ;[1 1 1] End Game
    (bind _asbp_ctr_player (cast `/Game/MyContent/Characters/BP_CTR_Player` (`GameplayStatics.GetPlayerPawn` 0)))
    (`self.Lever`)
    (`self.EndGame`)
    (`Widget.SetVisibility` (`/Game/MyContent/Characters/UI/UI_PlayerHUD.GameOver` (`/Game/MyContent/Characters/BP_CTR_Player.PlayerHUD` _asbp_ctr_player)) "Visible")))

(fn `UserConstructionScript`
  (`parent.UserConstructionScript`))