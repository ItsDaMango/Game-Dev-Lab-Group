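; BP_INT_SS_DoorB_Master is an interactible that opens and closes a group of B-type doors based on player proximity.
; When a BP_CTR_Player begins overlapping InteractCollision, it calls Open on every entry in the DoorsB array.
; When the player's overlap ends, it calls Reverse on the same doors.
; The construction script only runs the parent's logic.
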(event `self.InteractCollision.OnComponentBeginOverlap`
  (params (OverlappedComponent :type "PrimitiveComponent Object Reference") (OtherActor :type "Actor Object Reference") (OtherComp :type "PrimitiveComponent Object Reference") (OtherBodyIndex :type Integer) (bFromSweep :type Boolean) (SweepResult :type "HitResult Structure (by ref)"))
  (cast `/Game/MyContent/Characters/BP_CTR_Player` OtherActor)
  (for _array_element (`self.DoorsB`)
    (`self.Open` _array_element)))

(event `self.InteractCollision.OnComponentEndOverlap`
  (params (OverlappedComponent :type "PrimitiveComponent Object Reference") (OtherActor :type "Actor Object Reference") (OtherComp :type "PrimitiveComponent Object Reference") (OtherBodyIndex :type Integer))
  (cast `/Game/MyContent/Characters/BP_CTR_Player` OtherActor)
  (for _array_element (`self.DoorsB`)
    (`self.Reverse` _array_element)))

(fn `UserConstructionScript`
  (`parent.UserConstructionScript`))