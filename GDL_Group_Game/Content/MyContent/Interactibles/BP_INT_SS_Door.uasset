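; BP_INT_SS_Door is a switch interactible that feeds a key to a linked Door.
; Switching on or off runs the parent logic, then adds or removes a key on the Door, and both do nothing if the Door reference is invalid.
; Its OpenDoor and CloseDoor events are empty, and the TL_Door timeline play and reverse calls are disconnected leftovers that never run.
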(event `OpenDoor`)

(event `CloseDoor`)

(fn `SwitchedOff`
  (bind _door (`self.Door`)
    (:`then`
      (`parent.SwitchedOff`)
      (`/Game/MyContent/Mechanics/BP_DoorWithKeys.RemoveKey` _door true))
    (:`else`)))

(fn `SwitchedOn`
  (bind _door (`self.Door`)
    (:`then`
      (`parent.SwitchedOn`)
      (`/Game/MyContent/Mechanics/BP_DoorWithKeys.AddKey` _door true))
    (:`else`)))

(fn `UserConstructionScript`
  (`parent.UserConstructionScript`))