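; Interactable numpad switch that shows a password entry UI for a linked door.
; Switching on creates UI_Numpad with the password, door and player controller, then switches to UI-only input with a visible cursor.
; Switching off clears all widgets, restores game input, rebuilds the player HUD and calls RemoveKey on the door.
; Both actions require a valid Door, and Interact defers to the parent class.
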(event `self.ReceiveBeginPlay`
  (`parent.ReceiveBeginPlay`))

(fn `Interact`
  (`parent.Interact`))

(fn `SwitchedOff`
  (bind _returnvalue (`GameplayStatics.GetPlayerController` 0))
  (bind _door (`self.Door`)
    (:`then`
      (`WidgetLayoutLibrary.RemoveAllWidgets`)
      (`WidgetBlueprintLibrary.SetInputMode_GameOnly` _returnvalue)
      (set `PlayerController.bShowMouseCursor` false _returnvalue)
      (bind _asbp_ctr_player (cast `/Game/MyContent/Characters/BP_CTR_Player` (`GameplayStatics.GetPlayerPawn` 0)))
      (`/Game/MyContent/Characters/BP_CTR_Player.CreatePlayerHUD` _asbp_ctr_player)
      (`/Game/MyContent/Mechanics/BP_DoorWithKeys.RemoveKey` _door true))
    (:`else`)))

(fn `SwitchedOn`
  (bind _returnvalue (`GameplayStatics.GetPlayerController` 0))
  (`self.Door`
    (:`then`
      (bind _returnvalue_2 (`|CreateWidget` "/Game/MyContent/Characters/UI/UI_Numpad.UI_Numpad_C" null (`self.Password`)))
      (`UserWidget.AddToViewport` _returnvalue_2 0)
      (set `/Game/MyContent/Characters/UI/UI_Numpad.Door` (`self.Door`) _returnvalue_2)
      (set `/Game/MyContent/Characters/UI/UI_Numpad.PlayerController` _returnvalue _returnvalue_2)
      (`WidgetBlueprintLibrary.SetInputMode_UIOnlyEx` _returnvalue _returnvalue_2 "LockInFullscreen")
      (set `PlayerController.bShowMouseCursor` true _returnvalue))
    (:`else`)))

(fn `UserConstructionScript`
  (`parent.UserConstructionScript`))