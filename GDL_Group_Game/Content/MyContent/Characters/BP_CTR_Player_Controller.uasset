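; Player controller that routes Enhanced Input actions to the controlled BP_CTR_Player character.
; On BeginPlay it adds the locomotion and interact mapping contexts, then caches the pawn as PlayerRef.
; Camera rotation feeds yaw and pitch directly, while movement, jump, shooting, sprint, reload, interact and freeze shot call functions on the player.
; A FlipFlop alternates showing and hiding the inventory on each trigger.
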(event `self.ReceiveBeginPlay`
  ;[1 0.6732 0.3176] BeginPlay
  (`self.AddIMC` "/Game/MyContent/Characters/Input/IMC_Locomotion.IMC_Locomotion")
  (`self.AddIMC` "/Game/MyContent/Characters/Input/IMC_Interact.IMC_Interact")
  (bind _asbp_ctr_player (cast `/Game/MyContent/Characters/BP_CTR_Player` (`self.K2_GetPawn`)))
  (set `self.PlayerRef` _asbp_ctr_player))

(event `EnhancedInput|/Game/MyContent/Characters/Input/IA_Jump`
  (params (ActionValue :type Boolean) (ElapsedSeconds :type "Float (double-precision)") (TriggeredSeconds :type "Float (double-precision)") (InputAction :type "InputAction Object Reference" :default "/Game/MyContent/Characters/Input/IA_Jump.IA_Jump"))
  ;[1 1 1] Jumping
  (:`Triggered`
    (`/Game/MyContent/Characters/BP_CTR_Player.TryJump` (`self.PlayerRef`) ActionValue)))

(event `EnhancedInput|/Game/MyContent/Characters/Input/IA_Movement`
  (params (ActionValue :type "Vector2D Structure") (ElapsedSeconds :type "Float (double-precision)") (TriggeredSeconds :type "Float (double-precision)") (InputAction :type "InputAction Object Reference" :default "/Game/MyContent/Characters/Input/IA_Movement.IA_Movement"))
  ;[1 1 1] Movement
  (:`Triggered`
    (`/Game/MyContent/Characters/BP_CTR_Player.MovePlayer` (`self.PlayerRef`) ActionValue)))

(event `EnhancedInput|/Game/MyContent/Characters/Input/IA_CameraRotation`
  (params (ActionValue :type "Vector2D Structure") (ElapsedSeconds :type "Float (double-precision)") (TriggeredSeconds :type "Float (double-precision)") (InputAction :type "InputAction Object Reference" :default "/Game/MyContent/Characters/Input/IA_CameraRotation.IA_CameraRotation"))
  ;[1 1 1] Camera Rotation
  (:`Triggered`
    (`self.AddYawInput` ActionValue_X)
    (`self.AddPitchInput` ActionValue_Y)))

(event `EnhancedInput|/Game/MyContent/Characters/Input/IA_MainWeapon`
  (params (ActionValue :type Boolean) (ElapsedSeconds :type "Float (double-precision)") (TriggeredSeconds :type "Float (double-precision)") (InputAction :type "InputAction Object Reference" :default "/Game/MyContent/Characters/Input/IA_MainWeapon.IA_MainWeapon"))
  (bind _playerref (`self.PlayerRef`))
  ;[1 1 1] Shooting
  (:`Triggered`
    (if ActionValue
      (`/Game/MyContent/Characters/BP_CTR_Player.Start Shooting` _playerref)
      (else
        (`/Game/MyContent/Characters/BP_CTR_Player.StopShoot` _playerref)))))

(event `EnhancedInput|/Game/MyContent/Characters/Input/IA_Sprint`
  (params (ActionValue :type Boolean) (ElapsedSeconds :type "Float (double-precision)") (TriggeredSeconds :type "Float (double-precision)") (InputAction :type "InputAction Object Reference" :default "/Game/MyContent/Characters/Input/IA_Sprint.IA_Sprint"))
  (bind _playerref (`self.PlayerRef`))
  (:`Triggered`
    (if ActionValue
      (`/Game/MyContent/Characters/BP_CTR_Player.StartSprinting` _playerref)
      (else
        (`/Game/MyContent/Characters/BP_CTR_Player.StopSprinting` _playerref)))))

(event `EnhancedInput|/Game/MyContent/Characters/Input/IA_Interact`
  (params (ActionValue :type Boolean) (ElapsedSeconds :type "Float (double-precision)") (TriggeredSeconds :type "Float (double-precision)") (InputAction :type "InputAction Object Reference" :default "/Game/MyContent/Characters/Input/IA_Interact.IA_Interact"))
  ;[1 1 1] Interacting
  (:`Triggered`
    (if ActionValue
      (`/Game/MyContent/Characters/BP_CTR_Player.TryInteract` (`self.PlayerRef`)))))

(event `EnhancedInput|/Game/MyContent/Characters/Input/IA_Reload`
  (params (ActionValue :type Boolean) (ElapsedSeconds :type "Float (double-precision)") (TriggeredSeconds :type "Float (double-precision)") (InputAction :type "InputAction Object Reference" :default "/Game/MyContent/Characters/Input/IA_Reload.IA_Reload"))
  ;[1 1 1] reload
  (:`Triggered`
    (`/Game/MyContent/Characters/BP_CTR_Player.TryReload` (`self.PlayerRef`))
    (`KismetSystemLibrary.PrintString` "RELOAD")))

(event `EnhancedInput|/Game/MyContent/Characters/Input/IA_InventoryHideShow`
  (params (ActionValue :type Boolean) (ElapsedSeconds :type "Float (double-precision)") (TriggeredSeconds :type "Float (double-precision)") (InputAction :type "InputAction Object Reference" :default "/Game/MyContent/Characters/Input/IA_InventoryHideShow.IA_InventoryHideShow"))
  (bind _playerref (`self.PlayerRef`))
  ;[1 1 1] show/hide inventory on tab press
  (:`Triggered`
    (`/Engine/EditorBlueprintResources/StandardMacros.FlipFlop`
      (:`A`
        (`/Game/MyContent/Characters/BP_CTR_Player.ShowInventory` _playerref))
      (:`B`
        (`/Game/MyContent/Characters/BP_CTR_Player.HideInventory` _playerref)))))

(event `EnhancedInput|/Game/MyContent/Characters/Input/IA_FreezeEnemy`
  (params (ActionValue :type Boolean) (ElapsedSeconds :type "Float (double-precision)") (TriggeredSeconds :type "Float (double-precision)") (InputAction :type "InputAction Object Reference" :default "/Game/MyContent/Characters/Input/IA_FreezeEnemy.IA_FreezeEnemy"))
  (:`Triggered`
    (`/Game/MyContent/Characters/BP_CTR_Player.TryShootFreeze` (`self.PlayerRef`))))

(fn `AddIMC`
  (params (MappingContext :type "InputMappingContext Object Reference") (Priority :type Integer) (Options :type "ModifyContextOptions Structure"))
  (`EnhancedInputSubsystemInterface.AddMappingContext` (pcsubsystem `EnhancedInputLocalPlayerSubsystem` (`GameplayStatics.GetPlayerController` 0)) MappingContext Priority Options))

(fn `UserConstructionScript`)