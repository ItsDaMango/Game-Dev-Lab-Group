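; First-person player character with a hitscan laser rifle, reloading, aim zoom, sprinting, inventory, pause menu and a cooldown freeze ability for enemies and the last door.
; A looping timer from BeginPlay drives a camera sphere trace that sets the current interactable and HUD prompts.
; Shooting traces from muzzle along a camera cone, while timers handle fire rate, reload and cooldowns.
; HealthComponent events update the HUD, start combat music, or trigger ragdoll and death menu.
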(event `ZoomToAim`
  ;[0.7273 0.1745 1] zoom to aim and back timeline
  (bind (_direction _alpha) (`Timeline|TL_Aim` :!label _label)
    (:`Update`
      (`CameraComponent.SetFieldOfView` (`self.Camera`) (`KismetMathLibrary.Lerp` (`self.StandardZoomAngle`) (`self.AimZoomAngle`) _alpha)))))

(event `ZoomToStandard`
  ;[0.7273 0.1745 1] zoom to aim and back timeline
  (goto _label :!via `Reverse`))

(event `EnhancedInput|/Game/MyContent/Characters/Input/IA_PauseGame`
  (params (ActionValue :type Boolean) (ElapsedSeconds :type "Float (double-precision)") (TriggeredSeconds :type "Float (double-precision)") (InputAction :type "InputAction Object Reference" :default "/Game/MyContent/Characters/Input/IA_PauseGame.IA_PauseGame"))
  (:`Triggered`
    (`self.TogglePause`)))

(event `self.ReceiveBeginPlay`
  ;[1 0.09082 0.1605] BeginPlay
  ;[1 0.7422 0.3932] Adding Player UI
  (`self.SetPlayerHUD`)
  ;[0.5064 0.6228 1] Check If Interacting
  (`KismetSystemLibrary.K2_SetTimerDelegate` (`|CreateDelegate` :!event `InteractCheck`) 0.1 true)
  ;[1 1 1] init ammo UI
  (`self.RefreshUI`)
  ;[1 1 1] for progress bar
  (`self.UpdateHealthUI`)
  (`SceneComponent.SetVisibility` (`self.Weapon`) false false)
  (`GameplayStatics.PlaySound2D` "/Game/MyContent/SFX/StartGameSound.StartGameSound" 0.4 1.0 0.0 null null)
  (bind _returnvalue (`AddComponent|NODE_AddAudioComponent-2`))
  (bind _output_get (set `self.CombatMusic` _returnvalue))
  (`AudioComponent.Stop` _output_get))

(event `self.HealthComponent.OnTakeDamage`
  (params (Health :type "Float (double-precision)") (DamageCauser :type "Actor Object Reference"))
  (bind _returnvalue (`GameplayStatics.GetPlayerController` 0))
  (if (<= Health 0.0)
    (`self.Ragdoll`)
    (`PrimitiveComponent.SetCollisionResponseToAllChannels` (`self.Mesh`) "ECR_Ignore")
    (`KismetSystemLibrary.Delay` 1.5)
    (`UserWidget.AddToPlayerScreen` (`self.DeathMenu`) 0)
    (`WidgetBlueprintLibrary.SetInputMode_UIOnlyEx` _returnvalue null)
    (set `PlayerController.bShowMouseCursor` true _returnvalue)
    (else
      (`self.StartCombatMusic`))))

(event `self.HealthComponent.onHealthChanged`
  (params (NewHealth :type "Float (double-precision)"))
  (`self.UpdateHealthUI`))

(fn `AddAmmo`
  (params (Amount :type Integer))
  (returns (Success :type Boolean))
  (locals (L_PrevAmmo :type Integer))
  (bind _ammo (`self.Ammo`))
  (set `local.L_PrevAmmo` _ammo)
  (set `self.Ammo` (`KismetMathLibrary.Clamp` (+ _ammo Amount) 0 (`self.MaxAmmo`)))
  (`self.UpdateAmmoUI`)
  (return (!= (`self.Ammo`) (`local.L_PrevAmmo`))))

(fn `AddHealth`)

(fn `AddInput`
  (params (MappingContext :type "InputMappingContext Object Reference"))
  (`EnhancedInputSubsystemInterface.AddMappingContext` (pcsubsystem `EnhancedInputLocalPlayerSubsystem` (`GameplayStatics.GetPlayerController` 0)) MappingContext 0 (struct)))

(fn `CameraShake`
  (`GameplayStatics.PlayWorldCameraShake` "/Game/MyContent/Characters/BP_CameraShake.BP_CameraShake_C" (`self.K2_GetActorLocation`) 0.0 500.0))

(fn `ClearInteractable`
  (`self.CurrentInteractable`
    (:`then`
      (set `self.CurrentInteractable` null)
      (`/Game/MyContent/Characters/UI/UI_PlayerHUD.SetInteract` (`self.PlayerHUD`) false ""))
    (:`else`)))

(fn `CompleteReload`
  (`self.ReloadAmmo`)
  (set `self.IsReloading` false))

(fn `Cool Down Freeze`
  (set `self.FreezeHasHit` false)
  (set `self.FreezeOnCoolDown` true)
  (`Widget.SetVisibility` (`/Game/MyContent/Characters/UI/UI_PlayerHUD.Text_FreezeReady` (`self.PlayerHUD`)) "Hidden")
  (`KismetSystemLibrary.K2_SetTimerDelegate` (`|CreateDelegate` :!event `EndFreezeCoolDown`) (`self.FreezeCoolDownPeriod`)))

(fn `CoolDownShoot`
  (set `self.ShootOnCoolDown` true)
  (`KismetSystemLibrary.K2_SetTimerDelegate` (`|CreateDelegate` :!event `EndShootCoolDown`) (`self.FireRate`)))

(fn `CreatePlayerHUD`
  (bind _returnvalue (`|CreateWidget` "/Game/MyContent/Characters/UI/UI_PlayerHUD.UI_PlayerHUD_C" (`GameplayStatics.GetPlayerController` 0)))
  (bind _output_get (set `self.PlayerHUD` _returnvalue))
  (`UserWidget.AddToPlayerScreen` _output_get 0))

(fn `EndFreezeCoolDown`
  (set `self.FreezeOnCoolDown` false)
  (`Widget.SetVisibility` (`/Game/MyContent/Characters/UI/UI_PlayerHUD.Text_FreezeReady` (`self.PlayerHUD`)) "Visible")
  (bind _freezeemitter (`self.FreezeEmitter`)
    (:`then`
      ;[1 1 1] Destroy Sparks after freeze has finished
      (`ActorComponent.K2_DestroyComponent` _freezeemitter)
      (`self.CurrentEnemyToFreeze`
        (:`then`
          (set `self.CurrentEnemyToFreeze` null))
        (:`else`)))
    (:`else`)))

(fn `EndShootCoolDown`
  (set `self.ShootOnCoolDown` false))

(fn `HideInventory`
  (bind _returnvalue (`GameplayStatics.GetPlayerController` 0))
  (if (`self.ShowingInventory`)
    (set `self.ShowingInventory` false)
    (`Widget.SetVisibility` (`self.InventoryWidget`) "Hidden")
    (`WidgetBlueprintLibrary.SetInputMode_GameOnly` _returnvalue)
    (set `PlayerController.bShowMouseCursor` false _returnvalue)))

(fn `InteractCheck`
  (bind _txt_freezedoor (`/Game/MyContent/Characters/UI/UI_PlayerHUD.TXT_FreezeDoor` (`self.PlayerHUD`)))
  (bind _text_freezeready (`/Game/MyContent/Characters/UI/UI_PlayerHUD.Text_FreezeReady` (`self.PlayerHUD`)))
  (bind _txt_etointeract (`/Game/MyContent/Characters/UI/UI_PlayerHUD.TXT_EToInteract` (`self.PlayerHUD`)))
  (bind (_outhit _returnvalue) (`self.LineTraceFromCamera` (`self.InteractDistance`)))
  (if _returnvalue
    (`|ExecutionSequence`
      (:`then_0`
        (bind (_bblockinghit _binitialoverlap _time _distance _location _impactpoint _normal _impactnormal _physmat _hitactor) (`GameplayStatics.BreakHitResult` _outhit))
        ;[1 1 1] save if interactible was hit, else clear interactible
        (bind _asbp_interactible (cast `/Game/MyContent/Interactibles/BP_Interactible` _hitactor)
          (:`then`
            (`self.SetCurrentInteractable` _asbp_interactible)
            (`Widget.SetVisibility` _txt_etointeract "Visible")
            (cast `/Game/MyContent/Interactibles/BP_INT_SS_DoorB` _asbp_interactible))
          (:`CastFailed`
            (`self.ClearInteractable`)))
        (`Widget.SetVisibility` _txt_etointeract "Hidden"))
      (:`then_1`
        ;[1 1 1] IS Door
        (bind _asbp_int_ss_door_b (cast `/Game/MyContent/Interactibles/BP_INT_SS_DoorB` _hitactor)
          (:`then`
            (if (`/Game/MyContent/Interactibles/BP_INT_SS_DoorB.IsLastDoor` _asbp_int_ss_door_b)
              (`Widget.SetVisibility` _txt_freezedoor "Visible")
              (else
                (`Widget.SetVisibility` _txt_freezedoor "Hidden" :!label _label))))
          (:`CastFailed`
            (goto _label))))
      (:`then_2`
        (cast `/Game/MyContent/Characters/Enemies/BP_CTR_Enemy` _hitactor
          (:`then`
            (`Widget.SetVisibility` (`/Game/MyContent/Characters/UI/UI_PlayerHUD.TXT_Freeze` (`self.PlayerHUD`)) "Visible")
            (if (not (`self.FreezeOnCoolDown`))
              (`Widget.SetVisibility` _text_freezeready "Visible")
              (`Widget.SetVisibility` (`/Game/MyContent/Characters/UI/UI_PlayerHUD.IMG_Reticle_Ability` (`self.PlayerHUD`)) "Visible")
              (else
                (`Widget.SetVisibility` _text_freezeready "Hidden")
                (`Widget.SetVisibility` (`/Game/MyContent/Characters/UI/UI_PlayerHUD.IMG_Reticle_Ability` (`self.PlayerHUD`)) "Hidden"))))
          (:`CastFailed`
            (`Widget.SetVisibility` (`/Game/MyContent/Characters/UI/UI_PlayerHUD.IMG_Reticle_Ability` (`self.PlayerHUD`)) "Hidden")
            (`Widget.SetVisibility` (`/Game/MyContent/Characters/UI/UI_PlayerHUD.TXT_Freeze` (`self.PlayerHUD`)) "Hidden")))))
    (else
      ;[1 1 1] Failed
      (`Widget.SetVisibility` (`/Game/MyContent/Characters/UI/UI_PlayerHUD.IMG_Reticle_Interact` (`self.PlayerHUD`)) "Hidden")
      (`Widget.SetVisibility` (`/Game/MyContent/Characters/UI/UI_PlayerHUD.IMG_Reticle_Ability` (`self.PlayerHUD`)) "Hidden")
      (`Widget.SetVisibility` (`/Game/MyContent/Characters/UI/UI_PlayerHUD.TXT_Freeze` (`self.PlayerHUD`)) "Hidden")
      (`self.ClearInteractable`))))

(fn `MovePlayer`
  (params (Axis :type "Vector2D Structure"))
  (bind (_returnvalue_roll _returnvalue_pitch _returnvalue_yaw) (`KismetMathLibrary.BreakRotator` (`self.GetControlRotation`)))
  (bind _returnvalue (`KismetMathLibrary.MakeRotator` 0.0 0.0 _returnvalue_yaw))
  (`self.AddMovementInput` (`KismetMathLibrary.GetForwardVector` _returnvalue) Axis_X)
  (`self.AddMovementInput` (`KismetMathLibrary.GetRightVector` _returnvalue) Axis_Y))

(fn `NeedToReload`)

(fn `Ragdoll`
  (`self.DisableInput` null)
  (`PrimitiveComponent.SetCollisionEnabled` (`self.CapsuleComponent`) "NoCollision")
  (`PrimitiveComponent.SetCollisionEnabled` (`self.Arms`) "QueryAndPhysics")
  (`PrimitiveComponent.SetSimulatePhysics` (`self.Arms`) true)
  (`ActorComponent.SetActive` (`self.Camera`) false false)
  (`ActorComponent.SetActive` (`self.RagdollCam`) true false)
  (`SceneComponent.SetVisibility` (`self.Weapon`) false false))

(fn `RefreshUI`
  (`self.PlayerHUD`
    (:`then`
      (`self.UpdateAmmoUI`))
    (:`else`
      (`KismetSystemLibrary.K2_SetTimerDelegate` (`|CreateDelegate` :!event `RefreshUI`) 0.25))))

(fn `ReloadAmmo`
  (locals (L_ReloadAmount :type Integer))
  (bind _output_get (set `local.L_ReloadAmount` (`KismetMathLibrary.Clamp` (- (`self.MaxWeaponClip`) (`self.WeaponClip`)) 0 (`self.Ammo`))))
  (set `self.Ammo` (- (`self.Ammo`) _output_get))
  (set `self.WeaponClip` (+ (`self.WeaponClip`) (`local.L_ReloadAmount`)))
  (`self.UpdateAmmoUI`))

(fn `SetCurrentInteractable`
  (params (CurrentInteractable :type "/Game/MyContent/Interactibles/BP_Interactible Object Reference"))
  (bind _playerhud (`self.PlayerHUD`))
  (bind _output_get (set `self.CurrentInteractable` CurrentInteractable))
  (`/Engine/EditorBlueprintResources/StandardMacros.IsValid` _output_get
    (:`Is Valid`
      (bind _asbp_door_with_keys (cast `/Game/MyContent/Mechanics/BP_DoorWithKeys` _output_get)
        (:`then`
          (bind _allkeyscollected (`/Game/MyContent/Mechanics/BP_DoorWithKeys.AreAllKeysCollected` _asbp_door_with_keys))
          (if _allkeyscollected
            ;[1 1 1] Door is open so no mesage needed
            (`/Game/MyContent/Characters/UI/UI_PlayerHUD.SetInteract` (`self.PlayerHUD`) true "")
            (elif (`/Game/MyContent/Mechanics/BP_DoorWithKeys.IsPinProtected` _asbp_door_with_keys)
              ;[1 1 1] for doors with pin, say unlock with numpad first
              (`/Game/MyContent/Characters/UI/UI_PlayerHUD.SetInteract` _playerhud true "Unlock via numpad first")
              (else
                (`/Game/MyContent/Characters/UI/UI_PlayerHUD.SetInteract` _playerhud true "E to Interact")))))
        (:`CastFailed`
          ;[1 1 1] If Not a valid object, should be no message
          (`/Game/MyContent/Characters/UI/UI_PlayerHUD.SetInteract` (`self.PlayerHUD`) false ""))))
    (:`Is Not Valid`
      (`/Game/MyContent/Characters/UI/UI_PlayerHUD.SetInteract` (`self.PlayerHUD`) false ""))))

(fn `SetPlayerHUD`
  (bind _returnvalue (`|CreateWidget` "/Game/MyContent/Characters/UI/UI_PlayerHUD.UI_PlayerHUD_C"))
  (bind _output_get (set `self.PlayerHUD` _returnvalue))
  (`UserWidget.AddToPlayerScreen` _output_get 0)
  (bind _returnvalue_2 (`|CreateWidget` "/Game/MyContent/Characters/UI/UI_PauseMenu.UI_PauseMenu_C"))
  (set `self.PauseMenu` _returnvalue_2)
  (bind _returnvalue_3 (`|CreateWidget` "/Game/MyContent/Characters/UI/UI_DeathMenu.UI_DeathMenu_C"))
  (set `self.DeathMenu` _returnvalue_3)
  (bind _returnvalue_4 (`|CreateWidget` "/Game/MyContent/Characters/UI/UI_GameOver.UI_GameOver_C"))
  (set `self.GameOverMenu` _returnvalue_4))

(fn `ShootFreeze`
  (locals (LHitInfo :type "HitResult Structure"))
  (bind _camera (`self.Camera`))
  (`|ExecutionSequence`
    (:`then_0`
      (bind (_outhit _returnvalue) (`KismetSystemLibrary.SphereTraceSingle` (`SceneComponent.K2_GetComponentLocation` (`self.Muzzle`)) (+ (`SceneComponent.K2_GetComponentLocation` _camera) (* (`SceneComponent.GetForwardVector` _camera) (`self.FreezeDistance`))) 15.0 "TraceTypeQuery1"))
      (set `local.LHitInfo` _outhit)
      (if _returnvalue
        (bind (_bblockinghit _binitialoverlap _time _distance _location _impactpoint _normal _impactnormal _physmat _hitactor) (`GameplayStatics.BreakHitResult` _outhit))
        (bind _asbp_ctr_enemy (cast `/Game/MyContent/Characters/Enemies/BP_CTR_Enemy` _hitactor)
          (:`then`
            (set `self.FreezeHasHit` true)
            (bind _output_get (set `self.CurrentEnemyToFreeze` _asbp_ctr_enemy))
            (`|ExecutionSequence`
              (:`then_0`
                (`GameplayStatics.PlaySound2D` "/Game/MyContent/SFX/FreezeEnemy.FreezeEnemy" 1.0 1.0 0.0 null null))
              (:`then_1`
                (`/Game/MyContent/Characters/Enemies/BP_CTR_Enemy.FreezeEnemy` _output_get)
                (`self.Cool Down Freeze`))))
          (:`CastFailed`
            (bind _asbp_int_ss_door_b (cast `/Game/MyContent/Interactibles/BP_INT_SS_DoorB` _hitactor))
            (if (`/Game/MyContent/Interactibles/BP_INT_SS_DoorB.IsLastDoor` _asbp_int_ss_door_b)
              (set `self.FreezeHasHit` true)
              (`/Game/MyContent/Interactibles/BP_INT_SS_DoorB.StopDoor` _asbp_int_ss_door_b)
              (`self.Cool Down Freeze`))))))
    (:`then_1`
      (if (`self.FreezeHasHit`)
        (`KismetSystemLibrary.PrintString` "Iscooldowning?")
        (`self.Cool Down Freeze`)))))

(fn `ShootingEffects`
  (`|SpawnActorFromClass` "/Game/MyContent/Mechanics/BP_BulletTrail.BP_BulletTrail_C" (`KismetMathLibrary.MakeTransform` (`SceneComponent.K2_GetComponentLocation` (`self.Muzzle`)) (`KismetMathLibrary.MakeRotationFromAxes` (`SceneComponent.GetForwardVector` (`self.Camera`))) (2.0 2.0 2.0)) "AlwaysSpawn" "MultiplyWithRoot" self null)
  (`AnimInstance.Montage_Play` (`SkeletalMeshComponent.GetAnimInstance` (`self.Weapon`)) "/Game/MyContent/StaticMeshes/4_Weapons/SM_Gun_Fire.SM_Gun_Fire" 1.0 "Duration" 0.0 true)
  (`AnimInstance.Montage_Play` (`SkeletalMeshComponent.GetAnimInstance` (`self.Arms`)) "/Game/FPSAssaultPack/Animations/A_Arms_Rifle_Shoot01_Montage.A_Arms_Rifle_Shoot01_Montage" 1.0 "Duration" 0.0 true))

(fn `ShootWeapon`
  (locals (LHitInfo :type "HitResult Structure"))
  (bind _camera (`self.Camera`))
  (bind _playerhud (`self.PlayerHUD`))
  (`|ExecutionSequence`
    (:`then_0`
      (`GameplayStatics.PlaySound2D` "/Game/MyContent/SFX/LaserShot.LaserShot" 0.3 1.1 0.0 null null))
    (:`then_1`
      (`self.ShootingEffects`)
      (bind (_outhit _returnvalue) (`KismetSystemLibrary.LineTraceSingle` (`SceneComponent.K2_GetComponentLocation` (`self.Muzzle`)) (+ (`SceneComponent.K2_GetComponentLocation` _camera) (* (`KismetMathLibrary.RandomUnitVectorInConeInDegrees` (`SceneComponent.GetForwardVector` _camera) 1.0) (`self.WeaponRange`))) "TraceTypeQuery1"))
      (bind _output_get (set `local.LHitInfo` _outhit))
      (if _returnvalue
        (bind (_bblockinghit _binitialoverlap _time _distance _location _impactpoint _normal _impactnormal _physmat _hitactor) (`GameplayStatics.BreakHitResult` _outhit))
        (`GameplayStatics.ApplyPointDamage` _hitactor (`self.WeaponDamage`) _impactpoint _output_get null self)
        (`NiagaraFunctionLibrary.SpawnSystemAtLocation` "/Game/sA_Megapack_v1/sA_ShootingVfxPack/FX/NiagaraSystems/NS_Impact_2.NS_Impact_2" _impactpoint)
        (cast `/Game/MyContent/Characters/Enemies/BP_CTR_Enemy` _hitactor
          (:`then`
            (`GameplayStatics.PlaySoundAtLocation` "/Game/MyContent/SFX/Laser_Hit.Laser_Hit" _impactpoint (struct) 0.3 1.0 0.0 "/Game/MilitaryWeapDark/Sound/Attenuation/WeaponShot_att.WeaponShot_att" null null null)
            (`UserWidget.PlayAnimation` _playerhud (`/Game/MyContent/Characters/UI/UI_PlayerHUD.Anim_Hit` _playerhud) 0.0 1 "Forward" 1.0 false)
            (`self.StartCombatMusic`))
          (:`CastFailed`
            (`GameplayStatics.PlaySoundAtLocation` "/Game/MyContent/SFX/Impacts.Impacts" _impactpoint (struct) 1.0 1.0 0.0 "/Game/MilitaryWeapDark/Sound/Attenuation/ProjectileImpact_att.ProjectileImpact_att" null null null)))))
    (:`then_2`
      (`self.UseAmmo`)
      (`self.CoolDownShoot`))))

(fn `ShowInventory`
  (if (not (`self.ShowingInventory`))
    (set `self.ShowingInventory` true)
    (bind _inventorywidget (`self.InventoryWidget`)
      (:`then`
        (`Widget.SetVisibility` _inventorywidget "Visible"))
      (:`else`
        (bind _returnvalue (`|CreateWidget` "/Game/MyContent/Characters/UI/UI_Inventory.UI_Inventory_C" (`GameplayStatics.GetPlayerController` 0)))
        (bind _output_get (set `self.InventoryWidget` _returnvalue))
        (`UserWidget.AddToViewport` _output_get 2)
        (`WidgetBlueprintLibrary.SetInputMode_GameAndUIEx` (`GameplayStatics.GetPlayerController` 0) (`self.InventoryWidget`))
        (set `PlayerController.bShowMouseCursor` true (`GameplayStatics.GetPlayerController` 0))))))

(fn `Start Shooting`
  (`KismetSystemLibrary.K2_SetTimerDelegate` (`|CreateDelegate` :!event `TryShoot`) 0.01 true))

(fn `StartCombatMusic`
  (if (and (not (`self.InCombat`)) (not (`AudioComponent.IsPlaying` (`self.CombatMusic`))))
    (set `self.InCombat` true)
    (`AudioComponent.FadeIn` (`self.CombatMusic`) 4.0 1.0 0.0 "Linear")
    (`KismetSystemLibrary.K2_SetTimerDelegate` (`|CreateDelegate` :!event `StopCombatMusic`) 3.0)
    (else
      (`KismetSystemLibrary.K2_SetTimerDelegate` (`|CreateDelegate` :!event `StopCombatMusic`) 5.0))))

(fn `StartSprinting`
  (if (and (not (`self.IsSprinting`)) (not (`self.isAiming`)))
    (set `self.IsSprinting` true)
    (set `CharacterMovementComponent.MaxWalkSpeed` (`self.SprintSpeed`) (`self.CharacterMovement`))
    (`self.CameraShake`)))

(fn `StopAiming`
  (if (`self.isAiming`)
    (set `self.isAiming` false)
    (`self.ZoomToStandard`)))

(fn `StopCombatMusic`
  (if (and (`AudioComponent.IsPlaying` (`self.CombatMusic`)) (`self.InCombat`))
    (set `self.InCombat` false)
    (`AudioComponent.FadeOut` (`self.CombatMusic`) 3.0 0.0 "Linear")))

(fn `StopShoot`
  (`KismetSystemLibrary.K2_ClearTimer` null "TryShoot"))

(fn `StopSprinting`
  (if (`self.IsSprinting`)
    (set `self.IsSprinting` false)
    (set `CharacterMovementComponent.MaxWalkSpeed` (`self.WalkSpeed`) (`self.CharacterMovement`))
    (`KismetSystemLibrary.K2_ClearTimer` null "CameraShake")))

(fn `TogglePause`
  (`GameplayStatics.SetGamePaused` (not (`GameplayStatics.IsGamePaused`)))
  (if (`GameplayStatics.IsGamePaused`)
    (`UserWidget.AddToPlayerScreen` (`self.PauseMenu`) 0)
    (set `PlayerController.bShowMouseCursor` true (`GameplayStatics.GetPlayerController` 0))
    (`WidgetBlueprintLibrary.SetInputMode_GameAndUIEx` (`GameplayStatics.GetPlayerController` 0) (`self.PauseMenu`))
    (else
      (`Widget.RemoveFromParent` (`self.PauseMenu`))
      (set `PlayerController.bShowMouseCursor` false (`GameplayStatics.GetPlayerController` 0))
      (`WidgetBlueprintLibrary.SetInputMode_GameOnly` (`GameplayStatics.GetPlayerController` 0)))))

(fn `TryAim`
  (if (not (`self.isAiming`))
    (set `self.isAiming` true)
    (`self.ZoomToAim`)))

(fn `TryInteract`
  ;[1 1 1] check if null or has value. interact if able to
  (bind _currentinteractable (`self.CurrentInteractable`)
    (:`then`
      (`/Game/MyContent/Interactibles/BP_Interactible.Interact` _currentinteractable))
    (:`else`)))

(fn `TryJump`
  (params (GetJumping :type Boolean))
  (if GetJumping
    (`self.Jump`)
    (else
      (`self.StopJumping`))))

(fn `TryReload`
  ;[1 1 1] needs animation
  (if (and (not (`self.IsReloading`)) (not (`self.ShowingInventory`)) (not (== (`self.WeaponClip`) (`self.MaxWeaponClip`))) (not (`self.IsSprinting`)))
    (set `self.isReloading` true)
    (bind _returnvalue (`AnimInstance.Montage_Play` (`SkeletalMeshComponent.GetAnimInstance` (`self.Arms`)) "/Game/MilitaryWeapDark/Weapons/Anims/Reload_Rifle_Hip_W_Montage.Reload_Rifle_Hip_W_Montage" 1.0 "Duration" 0.0 true))
    (`KismetSystemLibrary.K2_SetTimerDelegate` (`|CreateDelegate` :!event `CompleteReload`) _returnvalue)))

(fn `TryShoot`
  ;[1 1 1] if false, show Reload needed animation
  (if (> (`self.WeaponClip`) 0)
    (if (and (not (`self.IsReloading`)) (not (`self.ShootOnCoolDown`)) (`self.EquipWeapon`) (not (`self.IsSprinting`)) (not (`self.ShowingInventory`)))
      (`self.ShootWeapon`))))

(fn `TryShootFreeze`
  (if (and (not (`self.FreezeOnCoolDown`)) (not (`self.FreezeHasHit`)))
    (`self.ShootFreeze`)))

(fn `UpdateAmmoUI`
  (bind _playerhud (`self.PlayerHUD`))
  (`/Game/MyContent/Characters/UI/UI_PlayerHUD.SetClip` _playerhud (`self.WeaponClip`))
  (`/Game/MyContent/Characters/UI/UI_PlayerHUD.SetAmmo` _playerhud (`self.Ammo`)))

(fn `UpdateHealthUI`
  (bind _playerhud (`self.PlayerHUD`)
    (:`then`
      (`/Game/MyContent/Characters/UI/UI_PlayerHUD.SetHealth` _playerhud (`self.HealthComponent`)))
    (:`else`)))

(fn `UseAmmo`
  (`/Engine/EditorBlueprintResources/StandardMacros.DecrementInt` (`self.WeaponClip`)
    (:`  `
      (`self.UpdateAmmoUI`))))

(fn `UserConstructionScript`
  (`parent.UserConstructionScript`))