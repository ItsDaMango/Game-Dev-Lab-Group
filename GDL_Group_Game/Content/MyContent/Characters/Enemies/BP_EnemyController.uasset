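; AI controller for enemy characters that runs the BT_Enemy behavior tree and turns perception sightings of the player into combat targets.
; A successfully sensed BP_CTR_Player is stored and written to the TargetActor blackboard key; losing perception does not clear it.
; The target is shared with enemies auto-assigned to the pawn's camp, with friend alerting disabled on those calls to prevent chained alerts.
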(event `self.ReceiveBeginPlay`
  (`self.RunBehaviorTree` "/Game/MyContent/Characters/Enemies/BT_Enemy.BT_Enemy"))

(event `self.AIPerception.OnTargetPerceptionUpdated`
  (params (Actor :type "Actor Object Reference") (Stimulus :type "AIStimulus Structure"))
  (bind _asbp_ctr_player (cast `/Game/MyContent/Characters/BP_CTR_Player` Actor))
  (if (`.bSuccessfullySensed` (break `AIStimulus` Stimulus))
    (`self.SetAITarget` _asbp_ctr_player)))

(fn `SetAITarget`
  (params (NewParam :type "Actor Object Reference") (AlerFriends :type Boolean :default true))
  (bind _output_get (set `self.CurentTarget` NewParam))
  (`BlackboardComponent.SetValueAsObject` (`AIBlueprintHelperLibrary.GetBlackboard` null) "TargetActor" _output_get)
  (if AlerFriends
    (`self.CurentTarget`
      (:`then`
        (bind _asbp_ctr_enemy (cast `/Game/MyContent/Characters/Enemies/BP_CTR_Enemy` (`self.K2_GetPawn`)))
        (for _array_element (`/Game/MyContent/Characters/Enemies/BP_EnemyCamp.Enemies(AutoAssigned)` (`/Game/MyContent/Characters/Enemies/BP_CTR_Enemy.Camp` _asbp_ctr_enemy))
          (`/Engine/EditorBlueprintResources/StandardMacros.IsValid` _array_element
            (:`Is Valid`
              (`/Game/MyContent/Characters/Enemies/BP_CTR_Enemy.SetTarget` _array_element (`self.CurentTarget`) false)))))
      (:`else`))))

(fn `UserConstructionScript`)