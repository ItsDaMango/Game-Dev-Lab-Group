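; BP_CTR_EnemyMedium is a medium enemy character that sets its range and health on BeginPlay, after the parent's setup.
; BasicAttack fires a hitscan line trace forward from FireFromLocation out to WeaponRange.
; Only on a hit, it applies point damage, spawns a small explosion at the fire location and plays rocket-launcher weapon and rifle body montages.
; That hit path returns the body montage duration scaled by FireRate.
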(event `self.ReceiveBeginPlay`
  (bind _healthcomponent (`self.HealthComponent`))
  (`parent.ReceiveBeginPlay`)
  (set `self.Range` 1000.0)
  (`/Game/MyContent/Core/BP_AC_Health.setHealth` _healthcomponent 200.0)
  (`/Game/MyContent/Core/BP_AC_Health.setMaxHealth` _healthcomponent 200.0))

(fn `BasicAttack`
  (returns (Duration :type "Float (double-precision)"))
  (bind _firefromlocation (`self.FireFromLocation`))
  (bind _returnvalue (`SceneComponent.K2_GetComponentLocation` _firefromlocation))
  (bind _returnvalue_2 (`SceneComponent.K2_GetComponentLocation` (`self.FireFromLocation`)))
  (bind (_outhit _returnvalue_3) (`KismetSystemLibrary.LineTraceSingle` _returnvalue (+ _returnvalue (* (`self.WeaponRange`) (`SceneComponent.GetForwardVector` _firefromlocation))) "TraceTypeQuery1"))
  (if _returnvalue_3
    (bind (_bblockinghit _binitialoverlap _time _distance _location _impactpoint _normal _impactnormal _physmat _hitactor) (`GameplayStatics.BreakHitResult` _outhit))
    (`GameplayStatics.ApplyPointDamage` _hitactor (`self.WeaponDamage`) _normal _outhit null self)
    (`GameplayStatics.SpawnEmitterAtLocation` "/Game/StarterContent/Particles/P_Explosion.P_Explosion" _returnvalue_2 (`KismetMathLibrary.MakeRotFromZ` _returnvalue_2) (0.2 0.2 0.2))
    (`AnimInstance.Montage_Play` (`SkeletalMeshComponent.GetAnimInstance` (`self.Weapon`)) "/Game/MilitaryWeapDark/Weapons/Anims/Fire_RocketLauncher_W_Montage.Fire_RocketLauncher_W_Montage" 1.0 "MontageLength" 0.0 true)
    (bind _returnvalue_4 (`AnimInstance.Montage_Play` (`SkeletalMeshComponent.GetAnimInstance` (`self.Mesh`)) "/Game/BattleDrone/Animations/BD_Fire_Rifle_Ironsights_Montage.BD_Fire_Rifle_Ironsights_Montage" 1.0 "Duration" 0.0 true))
    (return (* _returnvalue_4 (`self.FireRate`)))))

(fn `UserConstructionScript`
  (`parent.UserConstructionScript`))