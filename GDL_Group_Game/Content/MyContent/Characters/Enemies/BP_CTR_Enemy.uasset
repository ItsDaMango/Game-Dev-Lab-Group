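; Rifle-wielding enemy character that links itself to the nearest BP_EnemyCamp at construction.
; BasicAttack fires a hitscan trace for point damage, plays weapon and body montages, and returns montage length scaled by FireRate.
; Targets live on BP_EnemyController; taking damage targets the causer without alerting friends.
; At zero health, checked on damage and Tick, it ragdolls, catches fire and is destroyed; PostDeath spawns an impact effect.
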(event `self.ReceiveTick`
  (params (DeltaSeconds :type "Float (single-precision)"))
  (if (<= (`/Game/MyContent/Core/BP_AC_Health.health` (`self.HealthComponent`)) 0.0)
    (`self.SetTarget` (stale `self.HealthComponent.OnTakeDamage` DamageCauser) :!label _label)
    (if (<= (stale `self.HealthComponent.OnTakeDamage` Health) 0.0)
      (`PrimitiveComponent.SetSimulatePhysics` (`self.Mesh`) true)
      (`PrimitiveComponent.SetSimulatePhysics` (`self.SkeletalMesh`) true)
      (`KismetSystemLibrary.Delay` 0.2)
      (`GameplayStatics.SpawnEmitterAttached` "/Game/StarterContent/Particles/P_Fire.P_Fire" (`self.Mesh`) "Spine_02" (0.0 0.0 0.0) (struct) (0.2 0.2 0.2))
      (`KismetSystemLibrary.Delay` 1.0)
      (`self.K2_DestroyActor`))))

(event `self.HealthComponent.OnTakeDamage`
  (params (Health :type "Float (double-precision)") (DamageCauser :type "Actor Object Reference"))
  (goto _label))

(fn `BasicAttack`
  (returns (Duration :type "Float (double-precision)"))
  (bind _firefromlocation (`self.FireFromLocation`))
  (bind _returnvalue (`SceneComponent.K2_GetComponentLocation` _firefromlocation))
  (bind _outhit (`KismetSystemLibrary.LineTraceSingle` _returnvalue (+ _returnvalue (* (`self.WeaponRange`) (`SceneComponent.GetForwardVector` _firefromlocation))) "TraceTypeQuery1"))
  (bind (_bblockinghit _binitialoverlap _time _distance _location _impactpoint _normal _impactnormal _physmat _hitactor) (`GameplayStatics.BreakHitResult` _outhit))
  (`GameplayStatics.ApplyPointDamage` _hitactor (`self.WeaponDamage`) _normal _outhit null self)
  (`AnimInstance.Montage_Play` (`SkeletalMeshComponent.GetAnimInstance` (`self.Weapon`)) "/Game/FPSAssaultPack/Animations/Rifle/A_Rifle_Shoot01_Montage.A_Rifle_Shoot01_Montage" 1.0 "Duration" 0.0 true)
  (bind _returnvalue_2 (`AnimInstance.Montage_Play` (`SkeletalMeshComponent.GetAnimInstance` (`self.Mesh`)) "/Game/BattleDrone/Animations/BD_Fire_Rifle_Ironsights_Montage.BD_Fire_Rifle_Ironsights_Montage" 1.0 "Duration" 0.0 true))
  (return (* _returnvalue_2 (`self.FireRate`))))

(fn `GetCurrentTarget`
  (returns (CurentTarget :type "Actor Object Reference"))
  (bind _asbp_enemy_controller (cast `/Game/MyContent/Characters/Enemies/BP_EnemyController` (`self.GetController`)))
  (return (`/Game/MyContent/Characters/Enemies/BP_EnemyController.CurentTarget` _asbp_enemy_controller)))

(fn `PostDeath`
  (`GameplayStatics.SpawnEmitterAttached` "/Game/MilitaryWeapDark/FX/P_Impact_Metal_Large_01.P_Impact_Metal_Large_01" null "None" (`SceneComponent.GetSocketLocation` (`self.Mesh`) "thigh_r") (struct) (0.2 0.2 0.2)))

(fn `SetTarget`
  (params (Actor :type "Actor Object Reference") (AlerFriends :type Boolean))
  (bind _asbp_enemy_controller (cast `/Game/MyContent/Characters/Enemies/BP_EnemyController` (`self.GetController`)))
  (`/Game/MyContent/Characters/Enemies/BP_EnemyController.SetAITarget` _asbp_enemy_controller Actor AlerFriends))

(fn `UserConstructionScript`
  (`parent.UserConstructionScript`)
  (bind _outactors (`GameplayStatics.GetAllActorsOfClass` "/Game/MyContent/Characters/Enemies/BP_EnemyCamp.BP_EnemyCamp_C"))
  (bind _asbp_enemy_camp (cast `/Game/MyContent/Characters/Enemies/BP_EnemyCamp` (`.ReturnValue` (`GameplayStatics.FindNearestActor` (`self.K2_GetActorLocation`) _outactors))))
  (set `self.Camp` _asbp_enemy_camp))