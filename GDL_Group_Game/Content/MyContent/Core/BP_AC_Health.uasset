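; BP_AC_Health is an actor component that tracks current and maximum health for its owning actor.
; On BeginPlay it initializes both values and binds to the owner's point damage event; only that damage type is handled.
; Damage reduces health within a zero-to-max clamp, broadcasting OnHealthChanged through SetHealth, then OnTakeDamage with the damage causer.
; An optional debug flag draws health at the owner's location every tick.
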(event `self.ReceiveTick`
  (params (DeltaSeconds :type "Float (single-precision)"))
  ;[1 1 1] print health if debugHealth is turned on. For debugging purpose only
  (if (`self.debugHealth`)
    (`KismetSystemLibrary.DrawDebugString` (`Actor.K2_GetActorLocation` (`self.GetOwner`)) (`KismetStringLibrary.Conv_DoubleToString` (`self.Health`)) null (struct :`R` 1.0 :`A` 1.0))))

(event `self.ReceiveBeginPlay`
  (add `Actor.OnTakePointDamage` (`self.GetOwner`) (`|CreateDelegate` :!event `OnTakePointDamage`))
  (`self.setHealth` (`self.health`))
  (`self.setMaxHealth` (`self.maxHealth`)))

(fn `OnTakePointDamage`
  (params (DamagedActor :type "Actor Object Reference") (Damage :type "Float (single-precision)") (InstigatedBy :type "Controller Object Reference") (HitLocation :type "Vector Structure") (FHitComponent :type "PrimitiveComponent Object Reference") (BoneName :type Name) (ShotFromDirection :type "Vector Structure") (DamageType :type "DamageType Object Reference") (DamageCauser :type "Actor Object Reference"))
  (`self.setHealth` (`KismetMathLibrary.FClamp` (- (`self.Health`) Damage) 0.0 (`self.MaxHealth`)))
  (`self.OnTakeDamage` (`self.Health`) DamageCauser))

(fn `setHealth`
  (params (Health :type "Float (double-precision)"))
  (bind _output_get (set `self.health` (`KismetMathLibrary.FClamp` Health 0.0 (`self.maxHealth`))))
  (`self.onHealthChanged` _output_get))

(fn `setMaxHealth`
  (params (MaxHealth :type "Float (double-precision)"))
  (set `self.maxHealth` MaxHealth))